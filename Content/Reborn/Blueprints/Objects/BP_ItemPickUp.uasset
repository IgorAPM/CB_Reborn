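; Base item pickup actor that floats and spins, triggering an effect when the player's character touches it.
; A timeline started on BeginPlay bobs PickupMesh vertically and rotates it around yaw.
; On overlap with the first player's pawn, it casts to BP_BaseCharacter and passes it to ProcessPickupEffect.
; ProcessPickupEffect is empty here, serving as a hook for the actual effect.
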(event `self.ReceiveBeginPlay`
  (bind (_direction _movement _rotation) (`Timeline|Timeline_0` :!via `PlayFromStart`)
    (:`Update`
      (`SceneComponent.K2_SetRelativeLocation` (`self.PickupMesh`) (`KismetMathLibrary.MakeVector` 0.0 0.0 (* 20 _movement)) false false)
      (`SceneComponent.K2_SetRelativeRotation` (`self.PickupMesh`) (`KismetMathLibrary.MakeRotator` 0.0 0.0 (* -360 _rotation)) false false))))

(event `self.ReceiveActorBeginOverlap`
  (params (OtherActor :type "Actor Object Reference"))
  (bind _returnvalue (`Controller.K2_GetPawn` (`GameplayStatics.GetPlayerController` 0)))
  (if (== OtherActor _returnvalue)
    (bind _asbp_base_character (cast `/Game/Reborn/Blueprints/Characters/BP_BaseCharacter` _returnvalue))
    (`self.ProcessPickupEffect` _asbp_base_character)))

(event `ProcessPickupEffect`
  (params (ActorToAffect :type "/Game/Reborn/Blueprints/Characters/BP_BaseCharacter Object Reference")))

(fn `UserConstructionScript`)