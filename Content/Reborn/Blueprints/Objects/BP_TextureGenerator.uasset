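; Terrain generator actor that builds a procedural heightmap mesh from a noise material whenever its construction script runs.
; DrawTexture renders the noise material into a canvas render target with clamped addressing and nearest filtering.
; GenerateMesh reads that target pixel by pixel, turning red values times HeightScale into grid vertex heights with UVs and triangles.
; The procedural mesh is scaled by Width and Height, and its terrain material receives the same render texture.
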(event `DrawTexture`
  (`KismetRenderingLibrary.ClearRenderTarget2D` (`self.RenderTexture`))
  (bind (_canvas _size _context) (`KismetRenderingLibrary.BeginDrawCanvasToRenderTarget` (`self.RenderTexture`)))
  (`Canvas.K2_DrawMaterial` _canvas (`self.M_Ref`) (0.0 0.0) (`KismetMathLibrary.MakeVector2D` (`KismetMathLibrary.Conv_IntToDouble` (`self.Width`)) (`KismetMathLibrary.Conv_IntToDouble` (`self.Height`))) (0.0 0.0) (1.0 1.0) 0.0 (0.5 0.5))
  (`KismetRenderingLibrary.EndDrawCanvasToRenderTarget` _context)
  (`self.DrawMesh`))

(event `DrawMesh`
  (bind (_vertices1 _triangles1 _uvs1) (`self.GenerateMesh`))
  (`ProceduralMeshComponent.CreateMeshSection_LinearColor` :`self` (`self.ProceduralMesh`) :`Vertices` _vertices1 :`Triangles` _triangles1 :`UV0` _uvs1))

(fn `GenerateMesh`
  (returns (Vertices1 :type "Array of Vector Structure") (Triangles1 :type "Array of Integer") (Uvs1 :type "Array of Vector2D Structure"))
  (locals (Vertices :type "Array of Vector Structure") (Triangles :type "Array of Integer") (IndexY :type Integer) (IndexX :type Integer) (VertexIndex :type Integer) (Uvs :type "Array of Vector2D Structure") (TopLeftX :type "Float (double-precision)") (TopLeftY :type "Float (double-precision)"))
  (bind _vertexindex (`local.VertexIndex`))
  (set `local.TopLeftX` (/ (`KismetMathLibrary.Conv_IntToDouble` (- (`self.Width`) 1)) -2.0))
  (set `local.TopLeftY` (/ (`KismetMathLibrary.Conv_IntToDouble` (- (`self.Height`) 1)) 2.0))
  (for _index (range (+ (`self.Height`) 1))
    (set `local.IndexY` _index)
    (for _index_2 (range (+ (`self.Width`) 1))
      (set `local.IndexX` _index_2)
      (bind _returnvalue (`KismetRenderingLibrary.ReadRenderTargetRawPixel` (`self.RenderTexture`) (`local.IndexX`) (`local.IndexY`)))
      (`KismetArrayLibrary.Array_Add` (`local.Vertices`) (`KismetMathLibrary.MakeVector` (+ (`local.TopLeftX`) (`KismetMathLibrary.Conv_IntToDouble` (`local.IndexX`))) (- (`local.TopLeftY`) (`KismetMathLibrary.Conv_IntToDouble` (`local.IndexY`))) (* (break `LinearColor` _returnvalue) (`self.HeightScale`))))
      (`KismetArrayLibrary.Array_Add` (`local.Uvs`) (`KismetMathLibrary.MakeVector2D` (/ (`KismetMathLibrary.Conv_IntToDouble` (`local.IndexX`)) (`KismetMathLibrary.Conv_IntToDouble` (`self.Width`))) (/ (`KismetMathLibrary.Conv_IntToDouble` (`local.IndexY`)) (`KismetMathLibrary.Conv_IntToDouble` (`self.Height`)))))
      (if (and (< (`local.IndexX`) (- (`self.Width`) 1)) (< (`local.IndexY`) (- (`self.Height`) 1)))
        (for _array_element (`|MakeArray` (`local.VertexIndex`) (+ (`local.VertexIndex`) (`self.Width`) 1) (+ (`local.VertexIndex`) (`self.Width`)) (+ (`local.VertexIndex`) (`self.Width`) 1) _vertexindex (+ _vertexindex 1))
          (`KismetArrayLibrary.Array_Add` (`local.Triangles`) _array_element))
        (`/Engine/EditorBlueprintResources/StandardMacros.IncrementInt` (`local.VertexIndex`)))))
  (return (`local.Vertices`) (`local.Triangles`) (`local.Uvs`)))

(fn `UserConstructionScript`
  (bind _rendertexture (`self.RenderTexture`))
  (bind _returnvalue (`CanvasRenderTarget2D.CreateCanvasRenderTarget2D` "/Script/Engine.CanvasRenderTarget2D" (`self.Width`) (`self.Height`)))
  (set `self.RenderTexture` _returnvalue)
  (bind _returnvalue_2 (`KismetMaterialLibrary.CreateDynamicMaterialInstance` "/Game/Reborn/Materials/M_NoiseMaterial.M_NoiseMaterial"))
  (set `self.M_Ref` _returnvalue_2)
  (set `TextureRenderTarget2D.AddressX` "TA_Clamp" _rendertexture)
  (set `TextureRenderTarget2D.AddressY` "TA_Clamp" _rendertexture)
  (set `Texture.Filter` "TF_Nearest" _rendertexture)
  (`SceneComponent.SetRelativeScale3D` (`self.ProceduralMesh`) (`KismetMathLibrary.MakeVector` (`KismetMathLibrary.Conv_IntToDouble` (`self.Width`)) (`KismetMathLibrary.Conv_IntToDouble` (`self.Height`)) 1.0))
  (bind _returnvalue_3 (`PrimitiveComponent.CreateDynamicMaterialInstance` (`self.ProceduralMesh`) 0 "/Game/Reborn/Materials/M_TerrrainMaterial.M_TerrrainMaterial" "None"))
  (`MaterialInstanceDynamic.SetTextureParameterValue` _returnvalue_3 "RenderTexture" (`self.RenderTexture`))
  (`self.DrawTexture`))