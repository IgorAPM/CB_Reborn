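; Item pickup Blueprint that grants one extra projectile to the actor that collects it.
; It derives from a parent pickup class, which handles overlap and the base pickup effect.
; Its effect override passes a "+1" status with the PlusArrow type to the parent, increments the collector's ProjectileCount, then destroys itself.
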(event `self.ReceiveActorBeginOverlap`
  (params (OtherActor :type "Actor Object Reference"))
  (`parent.ReceiveActorBeginOverlap` OtherActor))

(event `self.ProcessPickupEffect`
  (params (ActorToAffect :type "/Game/Reborn/Blueprints/Characters/BP_BaseCharacter Object Reference") (StatusAmmount :type String) (StatusType :type Name))
  (`parent.ProcessPickupEffect` ActorToAffect (`KismetStringLibrary.Concat_StrStr` "+" "1") "PlusArrow")
  (set `/Game/Reborn/Blueprints/Characters/BP_BaseCharacter.ProjectileCount` (+ (`/Game/Reborn/Blueprints/Characters/BP_BaseCharacter.ProjectileCount` ActorToAffect) 1) ActorToAffect)
  (`self.K2_DestroyActor`))

(fn `UserConstructionScript`
  (`parent.UserConstructionScript`))