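; BP_ArrowProjectile is an arrow projectile that damages what it overlaps.
; On overlap with any actor other than its Instigator, it applies its Damage value, credited to the Instigator's controller, then destroys itself.
; An unconnected chain that would add a velocity-scaled impulse before destroying the arrow remains in the graph but never runs.
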(event `self.ReceiveActorBeginOverlap`
  (params (OtherActor :type "Actor Object Reference"))
  (if (not (== OtherActor (`self.Instigator`)))
    (`GameplayStatics.ApplyDamage` OtherActor (`self.Damage`) (`Pawn.GetController` (`self.Instigator`)) self)
    (`self.K2_DestroyActor`)))

(fn `UserConstructionScript`)