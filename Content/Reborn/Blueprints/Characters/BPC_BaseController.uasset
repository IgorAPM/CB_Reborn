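; BPC_BaseController is a player controller that relays movement and mouse aim to its BP_BaseCharacter pawn.
; On BeginPlay it caches the cast pawn and shows the mouse cursor.
; MoveForward and MoveRight axis inputs call the pawn's movement functions.
; Each tick it passes Aim a look-at rotation from the pawn toward the deprojected mouse world location, used directly without a trace or plane intersection.
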(event `self.ReceiveBeginPlay`
  (set `self.ControlledPawn` (cast `/Game/Reborn/Blueprints/Characters/BP_BaseCharacter` (`self.K2_GetPawn`) :!pure true))
  (set `self.bShowMouseCursor` true))

(event `InputAxis|MoveForward`
  (params (AxisValue :type "Float (single-precision)"))
  (`/Game/Reborn/Blueprints/Characters/BP_BaseCharacter.MoveForward` (`self.ControlledPawn`) AxisValue))

(event `InputAxis|MoveRight`
  (params (AxisValue :type "Float (single-precision)"))
  (`/Game/Reborn/Blueprints/Characters/BP_BaseCharacter.MoveSideways` (`self.ControlledPawn`) AxisValue))

(event `self.ReceiveTick`
  (params (DeltaSeconds :type "Float (single-precision)"))
  (bind _controlledpawn (`self.ControlledPawn`))
  (`/Game/Reborn/Blueprints/Characters/BP_BaseCharacter.Aim` _controlledpawn (`KismetMathLibrary.FindLookAtRotation` (`self.K2_GetActorLocation` _controlledpawn) (`self.DeprojectMousePositionToWorld`))))

(fn `UserConstructionScript`)