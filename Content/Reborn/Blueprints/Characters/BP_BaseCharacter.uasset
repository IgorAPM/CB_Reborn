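; Base bow-wielding character with world-axis movement, yaw-only aiming, jumping and health.
; Tick feeds its location to a location-based opacity parameter collection and health to a dynamic progress-bar material.
; Damage spawns a damage display, then triggers death or a flinch that blocks new attack montages.
; SpawnProjectile fires one arrow or a mirrored fan adding two per count, doubling the centre; the full-circle spread is unused.
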(event Custom|MoveForward
  (params (InputAxis :type Float%20%28single-precision%29))
  (Pawn|Input|AddMovementInput "1.000000,0.000000, 0" InputAxis false))

(event Custom|MoveSideways
  (params (InputAxis :type Float%20%28single-precision%29))
  (Pawn|Input|AddMovementInput "0.000000,1.000000, 0" InputAxis false))

(event Custom|Aim
  (params (NewRotation :type Rotator))
  (bind _returnvalue (Transformation|GetActorRotation))
  (if (> (Variables|Default|GetHealth) 0.0)
    (Transformation|SetActorRotation (Math|Rotator|MakeRotator (.roll _returnvalue) (.pitch _returnvalue) (.yaw NewRotation)))))

(event Custom|TryFireArrow
  (if (not (Variables|Default|GetIsFlinching))
    (if (not (Class|AnimInstance|MontageIsActive (Components|SkeletalMesh|GetAnimInstance (Variables|Character|GetMesh))))
      (Animation|PlayAnimMontage "/Game/ModularRPGHeroesPolyart/Animations/BowStance/AM_BaseBowAttackMontage.AM_BaseBowAttackMontage" 1.0 "Attack01"))))

(event Custom|DoJump
  (Character|Jump))

(event Custom|SpawnProjectile
  (if (> (Variables|Default|GetProjectileCount) 1)
    (bind _shotpositions1 (CallFunction|CalculateArrowShotPosFanned (Variables|Default|GetProjectileCount)))
    (for _array_element _shotpositions1
      (Game|SpawnActorfromClass "/Game/Reborn/Blueprints/Objects/BP_ArrowProjectile.BP_ArrowProjectile_C" _array_element "AlwaysSpawn" 0 25.0 self))
    (else
      (Game|SpawnActorfromClass "/Game/Reborn/Blueprints/Objects/BP_ArrowProjectile.BP_ArrowProjectile_C" (Transformation|GetWorldTransform (Variables|Default|GetForwardShotOffset)) "AlwaysSpawn" 0 25.0 self))))

(event EventBeginPlay)

(event Collision|EventActorBeginOverlap
  (params (OtherActor :type Actor%20Object%20Reference)))

(event EventTick
  (params (DeltaSeconds :type Float%20%28single-precision%29))
  (Rendering|Material|SetVectorParameterValue "/Game/Reborn/Materials/MPC_LocationBasedOpacity.MPC_LocationBasedOpacity" "Location" (Math|Conversions|ToLinearColor(Vector) (Transformation|GetActorLocation)) :!class /Script/Engine.KismetMaterialLibrary)
  (Rendering|Material|SetScalarParameterValue (Variables|Default|GetHealthMaterialRef) "Progress" (/ (Variables|Default|GetHealth) 1e+02) :!class /Script/Engine.MaterialInstanceDynamic))

(event Game|Damage|EventAnyDamage
  (params (Damage :type Float%20%28single-precision%29) (DamageType :type Damage%20Type%20Object%20Reference) (InstigatedBy :type Controller%20Object%20Reference) (DamageCauser :type Actor%20Object%20Reference))
  (Game|SpawnActorfromClass "/Game/Reborn/Blueprints/Objects/BP_DamageHolder.BP_DamageHolder_C" (Transformation|GetWorldTransform (Variables|Default|GetDamageViewer)) "Undefined" 0 "Fire" (Utilities|String|ToString(Float) Damage) 0)
  (bind _output_get (Variables|Default|SetHealth (- (Variables|Default|GetHealth) Damage)))
  (if (<= _output_get 0.0)
    (Utilities|FlowControl|DoOnce false
      (:Completed
        (Pawn|Components|CharacterMovement|DisableMovement (Variables|Character|GetCharacterMovement))
        (Components|Animation|PlayAnimation (Variables|Character|GetMesh) "/Game/ModularRPGHeroesPolyart/Animations/BowStance/Die_BowAnim.Die_BowAnim" false)
        (Variables|Default|SetIsFlinching false)))
    (else
      (Variables|Default|SetIsFlinching true)
      (bind _returnvalue (Animation|PlayAnimMontage "/Game/ModularRPGHeroesPolyart/Animations/BowStance/AM_GetHit.AM_GetHit" 1.0 "None"))
      (Utilities|FlowControl|Delay _returnvalue)
      (Variables|Default|SetIsFlinching false))))

(fn ConstructionScript
  (bind _returnvalue (Rendering|Material|CreateDynamicMaterialInstance (Variables|Default|GetPlane) 0 "/Game/RoboBars/Materials/ExamplesSurfaceCircle/MI_SimplePogress1.MI_SimplePogress1" "None" :!class /Script/Engine.PrimitiveComponent))
  (Variables|Default|SetHealthMaterialRef _returnvalue))

(fn CalculateArrowShotPosEvenly
  (params (ShotCount :type Integer))
  (bind _returnvalue (Transformation|GetActorLocation))
  (for _index (range 0 (- ShotCount 1))
    (Utilities|Array|Add (LocalVariables|GetShotPositions) (Math|Transform|MakeTransform (|(vector((CenterX+(InRadius*(cos(theta)))),(CenterY+(InRadius*(sin(Theta)))),CenterZ)) (.x _returnvalue) 1e+02 (+ (* _index (Math|Trig|DegreesToRadians (/ 3.6e+02 (Math|Conversions|ToFloat(Integer) ShotCount)))) (Math|Trig|DegreesToRadians (+ 0.0 (.yaw (Transformation|GetActorRotation))))) (.y _returnvalue) (.z _returnvalue)) (Math|Rotator|FindLookatRotation (Transformation|GetActorLocation) (|(vector((CenterX+(InRadius*(cos(theta)))),(CenterY+(InRadius*(sin(Theta)))),CenterZ)) (.x _returnvalue) 1e+02 (+ (* _index (Math|Trig|DegreesToRadians (/ 3.6e+02 (Math|Conversions|ToFloat(Integer) ShotCount)))) (Math|Trig|DegreesToRadians (+ 0.0 (.yaw (Transformation|GetActorRotation))))) (.y _returnvalue) (.z _returnvalue))))))
  (return (LocalVariables|GetShotPositions)))

(fn CalculateArrowShotPosFanned
  (params (ShotCount :type Integer))
  (bind _returnvalue (Transformation|GetActorLocation))
  (bind _returnvalue_2 (Transformation|GetActorLocation))
  (for _index (range 0 (- ShotCount 1))
    (Utilities|Array|Add (LocalVariables|GetShotPositions) (Math|Transform|MakeTransform (|(vector((CenterX+(InRadius*(cos(theta)))),(CenterY+(InRadius*(sin(Theta)))),CenterZ)) (.x _returnvalue) 1e+02 (+ (* _index (Math|Trig|DegreesToRadians (/ 9e+01 (Math|Conversions|ToFloat(Integer) ShotCount)))) (Math|Trig|DegreesToRadians (+ 0.0 (.yaw (Transformation|GetActorRotation))))) (.y _returnvalue) (.z _returnvalue)) (Math|Rotator|FindLookatRotation (Transformation|GetActorLocation) (|(vector((CenterX+(InRadius*(cos(theta)))),(CenterY+(InRadius*(sin(Theta)))),CenterZ)) (.x _returnvalue) 1e+02 (+ (* _index (Math|Trig|DegreesToRadians (/ 9e+01 (Math|Conversions|ToFloat(Integer) ShotCount)))) (Math|Trig|DegreesToRadians (+ 0.0 (.yaw (Transformation|GetActorRotation))))) (.y _returnvalue) (.z _returnvalue)))))
    (Utilities|Array|Add (LocalVariables|GetShotPositions) (Math|Transform|MakeTransform (|(vector((CenterX+(InRadius*(cos(theta)))),(CenterY+(InRadius*(sin(Theta)))),CenterZ)) (.x _returnvalue_2) 1e+02 (+ (* _index (Math|Trig|DegreesToRadians (/ -9e+01 (Math|Conversions|ToFloat(Integer) ShotCount)))) (Math|Trig|DegreesToRadians (+ 0.0 (.yaw (Transformation|GetActorRotation))))) (.y _returnvalue_2) (.z _returnvalue_2)) (Math|Rotator|FindLookatRotation (Transformation|GetActorLocation) (|(vector((CenterX+(InRadius*(cos(theta)))),(CenterY+(InRadius*(sin(Theta)))),CenterZ)) (.x _returnvalue_2) 1e+02 (+ (* _index (Math|Trig|DegreesToRadians (/ -9e+01 (Math|Conversions|ToFloat(Integer) ShotCount)))) (Math|Trig|DegreesToRadians (+ 0.0 (.yaw (Transformation|GetActorRotation))))) (.y _returnvalue_2) (.z _returnvalue_2))))))
  (return (LocalVariables|GetShotPositions)))